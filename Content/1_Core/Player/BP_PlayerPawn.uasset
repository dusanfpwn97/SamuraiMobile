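; BP_PlayerPawn is the player pawn, which equips a BP_Katana weapon when play begins.
; BeginPlay also caches the TargetArm's starting arm length and socket offset, and Tick defers to the parent class.
; Releasing the first touch destroys every SlashIndicator actor in the world, and the 1 key pauses the game.
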(event Custom|Test)

(event EventBeginPlay
  (bind _targetarm (Variables|Default|GetTargetArm))
  (Variables|Default|SetMaxTargetArmLength (Variables|/Script/Engine.SpringArmComponent|GetTargetArmLength _targetarm))
  (Variables|Default|SetInitialSocketOffset (Variables|/Script/Engine.SpringArmComponent|GetSocketOffset _targetarm))
  (Class|PlayerPawn|EquipNewWeapon "/Game/1_Core/Weapons/BP_Katana.BP_Katana_C"))

(event EventTick
  (params (DeltaSeconds :type Float%20%28single-precision%29))
  (|CallParentFunction DeltaSeconds))

(event Input|TouchEvents|Touch1
  (params (Key :type Key%20Structure :default "None"))
  (:Released
    (bind _outactors (Actor|GetAllActorsOfClass "/Script/Sam.SlashIndicator"))
    (for _array_element _outactors
      (Actor|DestroyActor _array_element))))

(event Input|KeyboardEvents|1
  (params (Key :type Key%20Structure :default "None"))
  (:Pressed
    (Game|SetGamePaused true)))

(fn ConstructionScript)