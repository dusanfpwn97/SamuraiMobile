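; Touch-controlled player pawn that dashes at enemies and attacks with a katana, using global time dilation for slow motion.
; Holding touch runs timelines that drive dash speed, and Tick slows time near the current target.
; Releasing plays the attack montage, whose Damage notify gates katana collision while a looping timer scales time by blade distance.
; SwordHit kills the enemy, selects the next target and triggers a hit-stop that Tick eases out.
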(event Custom|StartCheckSwordCollison
  (bind _currenttarget (Variables|Default|GetCurrentTarget))
  (Utilities|IsValid _currenttarget
    (:Is%20Valid
      (bind _asenemy_base (Utilities|Casting|CastToEnemyBase _currenttarget))
      (Variables|Default|SetAs%20Enemy%20Base _asenemy_base)
      (bind _returnvalue (Utilities|Time|SetTimerbyEvent (delegate Custom|CustomEvent_0) 0.002 true))
      (Variables|Default|SetNewVar_8 _returnvalue))))

(event Custom|SwordHit
  (params (NewParam :type Actor%20Object%20Reference))
  (Variables|Default|SetCurrentSlowDownDeltaTimeSum 0.0)
  (Variables|Default|SetNewVar_7 true)
  (bind _asenemy_base (Utilities|Casting|CastToEnemyBase NewParam))
  (Class|EnemyBase|Die _asenemy_base)
  (Class|PlayerPawn|SetNextTarget)
  (Utilities|Time|SetGlobalTimeDilation 0.004))

(event Custom|UpdateSlowMo
  (params (Delta :type Float%20%28double-precision%29)))

(event Custom|CheckEndAttack
  (if (Variables|Default|GetNewVar_7)
    (bind _output_get (Variables|Default|SetCurrentSlowDownDeltaTimeSum (+ (Variables|Default|GetCurrentSlowDownDeltaTimeSum) (Utilities|Time|GetWorldDeltaSeconds))))
    (if (> _output_get 0.0003)
      (Utilities|Time|SetGlobalTimeDilation (Math|Float|MapRangeClamped _output_get 0.0003 0.001 0.01 1.0))
      (Variables|Default|SetCurrentSpeed (* (Variables|Default|GetBaseSpeed) (Math|Float|MapRangeClamped _output_get 0.0003 0.001 0.01 1.0)))
      (if (> _output_get 0.001)
        (Variables|Default|SetNewVar_7 false)))))

(event Custom|StopCheckSwordCollison
  (Utilities|Time|ClearandInvalidateTimerbyHandle (Variables|Default|GetNewVar_8)))

(event Custom|CustomEvent_0
  (bind _returnvalue (Class|BaseWeapon|GetClosestCollisionDistance (Variables|Default|GetCurrentWeapon) (Variables|Default|GetCurrentTarget)))
  (if (Math|Boolean|ANDBoolean (< _returnvalue 3e+02) (not (Variables|Default|GetUsedSlowMoForCurrentAttack)) (Variables|Default|GetIsInDamangeWindow) (not (Variables|Default|GetNewVar_7)))
    (Utilities|Time|SetGlobalTimeDilation (Math|Float|MapRangeClamped _returnvalue 2e+02 1e+02 1.0 0.4))))

(event EventBeginPlay
  (bind _targetarm (Variables|Default|GetTargetArm))
  (Variables|Default|SetMaxTargetArmLength (Variables|/Script/Engine.SpringArmComponent|GetTargetArmLength _targetarm))
  (Variables|Default|SetNewVar_0 (Variables|/Script/Engine.SpringArmComponent|GetSocketOffset _targetarm))
  (Class|PlayerPawn|EquipNewWeapon "/Game/1_Core/Weapons/BP_Katana.BP_Katana_C"))

(event EventTick
  (params (DeltaSeconds :type Float%20%28single-precision%29))
  (bind _currenttarget (Variables|Default|GetCurrentTarget))
  (CallFunction|CheckEndAttack)
  (Utilities|IsValid _currenttarget
    (:Is%20Valid
      (if (not (Variables|Default|GetNewVar_1))
        (if (< (Transformation|GetDistanceTo _currenttarget self) 3.3e+02)
          (if (Variables|Default|GetNewVar_2)
            (Utilities|Time|SetGlobalTimeDilation 0.03)
            (Variables|Default|SetNewVar_2 false)
            (Variables|Default|SetCurrentSpeed (Variables|Default|GetBaseSpeed)))
          (elif (not (Variables|Default|GetNewVar_2))
            (Utilities|Time|SetGlobalTimeDilation 1.0)
            (Variables|Default|SetNewVar_2 true)))))))

(event Input|TouchEvents|Touch1
  (params (Key :type Key%20Structure :default "None"))
  (:Pressed
    (Variables|Default|SetNewVar_1 false)
    (Default|CallOnStartedDashing)
    (Variables|Default|SetIsChargingDash true)
    (Animation|Montage|PlayMontage (Variables|Character|GetMesh) "/Game/Animations/Player/GhostSamurai_APose_Attack01_3_InplaceStart_Montage.GhostSamurai_APose_Attack01_3_InplaceStart_Montage"
      (:then
        (bind _newtrack_0 (Timeline|Timeline_0 PlayFromStart)
          (:Update
            (Variables|Default|SetCurrentSpeed (* (Variables|Default|GetBaseSpeed) _newtrack_0)))
          (:Finished
            (Variables|Default|SetIsDashing true)
            (Variables|Default|SetIsChargingDash false)
            (bind _newtrack_0_2 (Timeline|Timeline_1 PlayFromStart)
              (:Update
                (if (Variables|Default|GetIsDashing)
                  (Variables|Default|SetCurrentSpeed (* _newtrack_0_2 (Variables|Default|GetBaseSpeed)))))))))))
  (:Released
    (Variables|Default|SetIsDashing false)
    (Variables|Default|SetNewVar_7 false)
    (Variables|Default|SetIsChargingDash false)
    (Variables|Default|SetNewVar_1 true)
    (Utilities|Time|SetGlobalTimeDilation 1.0)
    (Variables|Default|SetLastSlowMO 1.0)
    (Variables|Default|SetUsedSlowMoForCurrentAttack false)
    (Variables|Default|SetCurrentSlowDownDeltaTimeSum 0.0)
    (Variables|Default|SetCurrentSpeed 0.0)
    (Default|CallOnStartedAttacking)
    (bind _notifyname (Animation|Montage|PlayMontage (Variables|Character|GetMesh) "/Game/Animations/Player/GhostSamurai_APose_Attack01_1_ALL_Root_Montage.GhostSamurai_APose_Attack01_1_ALL_Root_Montage" 0.75)
      (:then
        (CallFunction|StartCheckSwordCollison)
        (Variables|Default|SetIsAnimatingAttack true))
      (:OnCompleted
        (CallFunction|StopCheckSwordCollison)
        (Variables|Default|SetIsAnimatingAttack false))
      (:OnNotifyBegin
        (switch name _notifyname
          (:damage
            (Variables|Default|SetIsInDamangeWindow true)
            (bind _asbp_katana (Utilities|Casting|CastToBP_Katana (Variables|Default|GetCurrentWeapon)))
            (Default|StartCheckingCollision _asbp_katana))))
      (:OnNotifyEnd
        (switch name _notifyname
          (:damage
            (Variables|Default|SetIsInDamangeWindow false)
            (bind _asbp_katana_2 (Utilities|Casting|CastToBP_Katana (Variables|Default|GetCurrentWeapon)))
            (Default|StopCheckingCollision _asbp_katana_2)))))))

(fn ConstructionScript)