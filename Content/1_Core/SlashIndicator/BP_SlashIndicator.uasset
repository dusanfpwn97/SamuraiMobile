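; BP_SlashIndicator is an actor that shows a moving indicator, by its name for a slash, oriented to the player's view.
; On BeginPlay a timeline lerps the Moving component from its starting world location to the Goal component's current location.
; Every tick the actor copies the first player pawn's control rotation.
; The start point is cached once in world space, while the Goal location is re-read on each timeline update.
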(event EventBeginPlay
  (bind _moving (Variables|Default|GetMoving))
  (Variables|Default|SetStartingLoc (Transformation|GetWorldLocation _moving))
  (bind _newtrack_0 (Timeline|Timeline_0 PlayFromStart)
    (:Update
      (Transformation|SetWorldLocation _moving (Math|Vector|Lerp(Vector) (Variables|Default|GetStartingLoc) (Transformation|GetWorldLocation (Variables|Default|GetGoal)) _newtrack_0) false false))))

(event Collision|EventActorBeginOverlap
  (params (OtherActor :type Actor%20Object%20Reference)))

(event EventTick
  (params (DeltaSeconds :type Float%20%28single-precision%29))
  (|CallParentFunction DeltaSeconds)
  (Transformation|SetActorRotation (Pawn|GetControlRotation (Game|Player|GetPlayerPawn 0) :!class /Script/Engine.Pawn)))

(fn ConstructionScript)